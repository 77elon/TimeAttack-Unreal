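; Race tracker Blueprint that runs a lap-based checkpoint course and hands its settings to MyPlayerController.
; At BeginPlay it copies lap count, save slot, map name and medal times to the controller, numbers the checkpoints, binds their cleared events and starts music.
; Each clear plays a sound, activates the next checkpoint's particles and trigger, and updates the respawn point.
; The final checkpoint updates the lap and either loops or flags race completion, triggering Restart.
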(event Custom|ApplySettings
  (bind _controllerreference (Variables|Default|GetControllerReference))
  ;[1 1 1] Apply User Settings at Game Start
  (Variables|/Game/BluePrints/MyPlayerController.MyPlayerController_C|SetMaxLaps _controllerreference (Variables|CustomSettings|GetMaxLaps))
  (Variables|/Game/BluePrints/MyPlayerController.MyPlayerController_C|SetSaveSlot _controllerreference (Variables|CustomSettings|GetSaveGameName))
  (Variables|/Game/BluePrints/MyPlayerController.MyPlayerController_C|SetNameOfMap _controllerreference (Variables|CustomSettings|GetNameOfLap))
  (CallFunction|UpdateTimes)
  (Default|StartGameSetup _controllerreference))

(event Custom|StartSequence
  (bind _checkpoints (Variables|CheckPoints|GetCheckPoints))
  ;[1 1 1] Start Sequence / Get all CheckPoints, Activate the First Checkpoint
  (for (_array_element _array_index) (Variables|CheckPoints|GetCheckPoints)
    (Variables|/Game/BluePrints/CheckPoint.CheckPoint_C|SetCheckPointNumber _array_element (+ _array_index 1))
    (Variables|Default|SetTotalCheckPoints (Utilities|Array|Length _checkpoints))
    (CallFunction|ActivateCheckPoint (Utilities|Array|Get(acopy) _checkpoints))
    (for _array_element_2 (Variables|CheckPoints|GetCheckPoints)
      (EventDispatchers|BindEventtoCheckPointCleared _array_element_2 (delegate Custom|CheckPointsCleared))
      (Audio|Components|Audio|Play (Variables|/Script/Engine.AmbientSound|GetAudioComponent (Variables|CustomSettings|GetLevelMusic)) 0.0))))

(event Custom|CheckPointsCleared
  (params (NextCheckPoint :type Integer))
  (bind _controllerreference (Variables|Default|GetControllerReference))
  ;[1 1 1] if CheckPoint Cleared...
  (CallFunction|LapCheck NextCheckPoint)
  (Audio|Components|Audio|Play (Variables|/Script/Engine.AmbientSound|GetAudioComponent (Variables|CustomSettings|GetCheckPointSoundFX)) 0.0)
  (if (Variables|/Game/BluePrints/MyPlayerController.MyPlayerController_C|GetRaceComplete _controllerreference)
    (Default|Restart _controllerreference)))

(event EventBeginPlay
  ;[1 1 1] BeginPlay / Custom Event Calling
  (bind _asmy_player_controller (Utilities|Casting|CastToMyPlayerController (Game|GetPlayerController 0)))
  (Variables|Default|SetControllerReference _asmy_player_controller)
  (CallFunction|ApplySettings)
  (CallFunction|StartSequence))

(fn ConstructionScript)

(fn UpdateTimes
  (bind _controllerreference (Variables|Default|GetControllerReference))
  ;[1 1 1] Pass User Settings
  (Variables|/Game/BluePrints/MyPlayerController.MyPlayerController_C|SetGoldTime _controllerreference (Variables|CustomSettings|GetGoldTime))
  (Variables|/Game/BluePrints/MyPlayerController.MyPlayerController_C|SetSilverTime _controllerreference (Variables|CustomSettings|GetSilverTime))
  (Variables|/Game/BluePrints/MyPlayerController.MyPlayerController_C|SetBronzeTime _controllerreference (Variables|CustomSettings|GetBronzeTime))
  (Variables|/Game/BluePrints/MyPlayerController.MyPlayerController_C|SetDefaultBestLapTime _controllerreference (Variables|CustomSettings|GetDefaultBestLap))
  (Variables|/Game/BluePrints/MyPlayerController.MyPlayerController_C|SetDefaultBestRaceTime _controllerreference (Variables|CustomSettings|GetDefaultBestTime)))

(fn LapCheck
  (params (CheckPoint :type Integer))
  ;[1 1 1] Lap Check
  (bind _output_get (LocalVariables|SetLocalCheckPoint CheckPoint))
  (if (== _output_get (Variables|Default|GetTotalCheckPoints))
    (bind _isracecompleted (CallFunction|RaceCompleteCheck))
    (if _isracecompleted
      _
      (else
        (CallFunction|ActivateCheckPoint (Utilities|Array|Get(acopy) (Variables|CheckPoints|GetCheckPoints)))))
    (Default|UpdateLap (Variables|Default|GetControllerReference))
    (else
      (CallFunction|ActivateCheckPoint (Utilities|Array|Get(acopy) (Variables|CheckPoints|GetCheckPoints) (LocalVariables|GetLocalCheckPoint)))))
  (Variables|/Game/BluePrints/MyPlayerController.MyPlayerController_C|SetRespawnLocation (Variables|Default|GetControllerReference) (Transformation|GetActorTransform (Utilities|Array|Get(acopy) (Variables|CheckPoints|GetCheckPoints) (- (LocalVariables|GetLocalCheckPoint) 1)))))

(fn ActivateCheckPoint
  (params (NextCheckPoint :type Check%20Point%20Object%20Reference))
  ;[1 1 1] Activate Next CheckPoint
  (Development|SetHiddeninGame (Variables|/Game/BluePrints/CheckPoint.CheckPoint_C|GetParticleSystem NextCheckPoint) false false)
  (Variables|/Script/Engine.PrimitiveComponent|SetbGenerateOverlapEvents (Variables|/Game/BluePrints/CheckPoint.CheckPoint_C|GetTrigger NextCheckPoint) true))

(fn RaceCompleteCheck
  (bind _controllerreference (Variables|Default|GetControllerReference))
  (bind _controllerreference_2 (Variables|Default|GetControllerReference))
  ;[1 1 1] Race Complete Check
  (if (>= (Variables|/Game/BluePrints/MyPlayerController.MyPlayerController_C|GetActualLap _controllerreference) (Variables|/Game/BluePrints/MyPlayerController.MyPlayerController_C|GetMaxLaps _controllerreference))
    (bind _output_get (Variables|/Game/BluePrints/MyPlayerController.MyPlayerController_C|SetRaceComplete _controllerreference_2 true))
    (LocalVariables|SetLocalCompleted _output_get)
    (else
      (bind _output_get_2 (Variables|/Game/BluePrints/MyPlayerController.MyPlayerController_C|SetRaceComplete _controllerreference_2 false))
      (LocalVariables|SetLocalCompleted _output_get_2)))
  (return (LocalVariables|GetLocalCompleted)))